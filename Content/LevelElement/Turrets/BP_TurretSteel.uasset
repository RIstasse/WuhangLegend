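; BP_TurretSteel is a turret level element Blueprint that handles the placement of the steel turret.
; Its PlaceTurretSteel event sets the Placed flag and enables query and physics collision on the BasePillier component.
; BeginPlay, ActorBeginOverlap and the construction script only call the parent class, and Tick is disabled.
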(event Custom|PlaceTurretSteel
  (Variables|Default|SetPlaced true)
  (Collision|SetCollisionEnabled (Variables|Default|GetBase_Pillier) "QueryAndPhysics"))

(event EventBeginPlay
  (|CallParentFunction))

(event Collision|EventActorBeginOverlap
  (params (OtherActor :type Actor%20Object%20Reference))
  (|CallParentFunction 0))

(event EventTick
  (params (DeltaSeconds :type Float%20%28single-precision%29))
  (|CallParentFunction DeltaSeconds) ; This node is disabled and will not be called.\nDrag off pins to build functionality.
)

(fn ConstructionScript
  (|CallParentFunction))