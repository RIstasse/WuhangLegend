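; Earth turret Blueprint that deals periodic area damage to enemies within its detection zone.
; OverlapDetection adds and removes BP_EnemyParent actors in the EnemyInRange list as they enter and leave.
; BeginPlay starts a looping Cooldown timer and runs a damage pass over that list, which each timer tick repeats.
; PlaceTurretEarth flags the turret as placed and enables pillar collision, though damage does not check that flag.
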(event OnComponentBeginOverlap(OverlapDetection)
  (params (OverlappedComponent :type Primitive%20Component%20Object%20Reference) (OtherActor :type Actor%20Object%20Reference) (OtherComp :type Primitive%20Component%20Object%20Reference) (OtherBodyIndex :type Integer) (bFromSweep :type Boolean) (SweepResult :type Hit%20Result%20Structure%20%28by%20ref%29))
  ;[1 1 1] Detecte les ennemis dans sa zone
  (bind _asbp_enemy_parent (Utilities|Casting|CastToBP_EnemyParent OtherActor))
  (Utilities|Array|Add (Variables|Default|GetEnemyInRange) _asbp_enemy_parent))

(event OnComponentEndOverlap(OverlapDetection)
  (params (OverlappedComponent :type Primitive%20Component%20Object%20Reference) (OtherActor :type Actor%20Object%20Reference) (OtherComp :type Primitive%20Component%20Object%20Reference) (OtherBodyIndex :type Integer))
  (bind _enemyinrange (Variables|Default|GetEnemyInRange))
  ;[1 1 1] Detecte les ennemis dans sa zone
  (bind _asbp_enemy_parent (Utilities|Casting|CastToBP_EnemyParent OtherActor))
  (if (Utilities|Array|ContainsItem _enemyinrange _asbp_enemy_parent)
    (Utilities|Array|RemoveItem _enemyinrange _asbp_enemy_parent)))

(event Custom|PlaceTurretEarth
  (Variables|Default|SetPlaced true)
  (Collision|SetCollisionEnabled (Variables|Default|GetBase_Pillier) "QueryAndPhysics"))

(event Custom|DealDamage
  ;[1 1 1] Dégât de zone
  (for _array_element (Variables|Default|GetEnemyInRange)
    (Game|Damage|ApplyDamage _array_element (Variables|Default|GetDamage) 0 0)))

(event EventTick
  (params (DeltaSeconds :type Float%20%28single-precision%29))
  (|CallParentFunction DeltaSeconds) ; This node is disabled and will not be called.\nDrag off pins to build functionality.
)

(event EventBeginPlay
  ;[1 1 1] Dégât de zone
  (Utilities|Time|SetTimerbyEvent (delegate Custom|DealDamage) (Variables|Default|GetCooldown) true)
  (for _array_element (Variables|Default|GetEnemyInRange)
    (Game|Damage|ApplyDamage _array_element (Variables|Default|GetDamage) 0 0)))

(fn ConstructionScript
  (|CallParentFunction))