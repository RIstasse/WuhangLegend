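; Parent turret Blueprint that auto-targets and shoots enemies, following the mouse cursor over the ground until placed.
; Overlap detection maintains an in-range enemy list, selecting the first entry and reselecting when the target leaves or dies.
; A gated, self-recalling Delay loop interpolates the turret's rotation toward the target and triggers delayed single or three-way spread projectile shots.
; DamageAura is an empty stub.
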(event OnComponentBeginOverlap(OverlapDetection)
  (params (OverlappedComponent :type Primitive%20Component%20Object%20Reference) (OtherActor :type Actor%20Object%20Reference) (OtherComp :type Primitive%20Component%20Object%20Reference) (OtherBodyIndex :type Integer) (bFromSweep :type Boolean) (SweepResult :type Hit%20Result%20Structure%20%28by%20ref%29))
  ;[1 1 1] Detection de l'ennemi
  (bind _asbp_enemy_parent (Utilities|Casting|CastToBP_EnemyParent OtherActor))
  (Utilities|Array|Add (Variables|Default|GetTargetsInRange) _asbp_enemy_parent)
  (Utilities|IsValid (Variables|Default|GetTargetEnemyDetected)
    (:Is%20Not%20Valid
      (CallFunction|SelectTarget))))

(event OnComponentEndOverlap(OverlapDetection)
  (params (OverlappedComponent :type Primitive%20Component%20Object%20Reference) (OtherActor :type Actor%20Object%20Reference) (OtherComp :type Primitive%20Component%20Object%20Reference) (OtherBodyIndex :type Integer))
  (bind _targetsinrange (Variables|Default|GetTargetsInRange))
  ;[1 1 1] Detection de l'ennemi
  (bind _asbp_enemy_parent (Utilities|Casting|CastToBP_EnemyParent OtherActor))
  (if (Utilities|Array|ContainsItem _targetsinrange _asbp_enemy_parent)
    (Utilities|Array|RemoveItem _targetsinrange _asbp_enemy_parent)
    (if (== _asbp_enemy_parent (Variables|Default|GetTargetEnemyDetected))
      (Variables|Default|SetTargetEnemyDetected 0)
      (CallFunction|SelectTarget))))

(event Custom|Select%20Target
  (bind _targetsinrange (Variables|Default|GetTargetsInRange))
  ;[1 1 1] Selection de l'ennemi
  (if (Utilities|Array|IsValidIndex _targetsinrange)
    (Variables|Default|SetTargetEnemyDetected (Utilities|Array|Get(acopy) _targetsinrange (Variables|Default|GetZero)))
    (CallFunction|BeginAim)))

(event Custom|BeginAim
  ;[1 1 1] Vise
  (Utilities|FlowControl|Sequence
    (:then_0
      (goto _label Open))
    (:then_1
      (Utilities|FlowControl|Gate true :!label _label
        (:Exit
          (Utilities|IsValid (Variables|Default|GetTargetEnemyDetected)
            (:Is%20Valid
              (Utilities|FlowControl|Sequence
                (:then_0
                  ;[1 1 1] Permet de tirer / vérifie si la tour est celle de Bois ou non
                  (Utilities|FlowControl|Delay (Variables|Default|GetRateOfShoot))
                  (if (Variables|Default|GetDidShot3)
                    (CallFunction|Shot3 (Variables|Default|GetProjectyleType))
                    (else
                      (CallFunction|Shot (Variables|Default|GetProjectyleType)))))
                (:then_1
                  ;[1 1 1] Tourelle suit l'ennemi
                  (Variables|Default|SetTargetLocation (Transformation|GetActorLocation (Variables|Default|GetTargetEnemyDetected)))
                  (Transformation|SetRelativeRotation (Variables|Default|GetCube) (Math|Interpolation|RInterpTo (Variables|/Script/Engine.SceneComponent|GetRelativeRotation (Variables|Default|GetCube)) (Math|Rotator|MakeRotator 0.0 (.Pitch (Math|Rotator|BreakRotator (Math|Rotator|MakeRotfromX (Math|Transform|InverseTransformDirection (Transformation|GetActorTransform) (- (Variables|Default|GetTargetLocation) (Transformation|GetWorldLocation (Variables|Default|GetCube))))))) (.Yaw (Math|Rotator|BreakRotator (Math|Rotator|MakeRotfromX (Math|Transform|InverseTransformDirection (Transformation|GetActorTransform) (- (Variables|Default|GetTargetLocation) (Transformation|GetWorldLocation (Variables|Default|GetCube)))))))) (Utilities|Time|GetWorldDeltaSeconds) (Variables|Default|GetRotation%20Speed)) false false)
                  (Utilities|FlowControl|Delay (Utilities|Time|GetWorldDeltaSeconds))
                  (CallFunction|ContinueAim))))
            (:Is%20Not%20Valid
              (CallFunction|CancelAim))))))))

(event Custom|ContinueAim
  (bind _targetsinrange (Variables|Default|GetTargetsInRange))
  ;[1 1 1] Vise
  (Utilities|IsValid (Variables|Default|GetTargetEnemyDetected)
    (:Is%20Valid
      (if (Variables|/Game/Ennemis/BP_EnemyParent.BP_EnemyParent_C|GetAlive (Variables|Default|GetTargetEnemyDetected))
        (Utilities|FlowControl|Gate true
          (:Exit
            (Utilities|IsValid (Variables|Default|GetTargetEnemyDetected)
              (:Is%20Valid
                (Utilities|FlowControl|Sequence
                  (:then_0
                    ;[1 1 1] Permet de tirer / vérifie si la tour est celle de Bois ou non
                    (Utilities|FlowControl|Delay (Variables|Default|GetRateOfShoot))
                    (if (Variables|Default|GetDidShot3)
                      (CallFunction|Shot3 (Variables|Default|GetProjectyleType))
                      (else
                        (CallFunction|Shot (Variables|Default|GetProjectyleType)))))
                  (:then_1
                    ;[1 1 1] Tourelle suit l'ennemi
                    (Variables|Default|SetTargetLocation (Transformation|GetActorLocation (Variables|Default|GetTargetEnemyDetected)))
                    (Transformation|SetRelativeRotation (Variables|Default|GetCube) (Math|Interpolation|RInterpTo (Variables|/Script/Engine.SceneComponent|GetRelativeRotation (Variables|Default|GetCube)) (Math|Rotator|MakeRotator 0.0 (.Pitch (Math|Rotator|BreakRotator (Math|Rotator|MakeRotfromX (Math|Transform|InverseTransformDirection (Transformation|GetActorTransform) (- (Variables|Default|GetTargetLocation) (Transformation|GetWorldLocation (Variables|Default|GetCube))))))) (.Yaw (Math|Rotator|BreakRotator (Math|Rotator|MakeRotfromX (Math|Transform|InverseTransformDirection (Transformation|GetActorTransform) (- (Variables|Default|GetTargetLocation) (Transformation|GetWorldLocation (Variables|Default|GetCube)))))))) (Utilities|Time|GetWorldDeltaSeconds) (Variables|Default|GetRotation%20Speed)) false false)
                    (Utilities|FlowControl|Delay (Utilities|Time|GetWorldDeltaSeconds))
                    (CallFunction|ContinueAim))))
              (:Is%20Not%20Valid
                (CallFunction|CancelAim :!label _label)))))
        (elif (Utilities|Array|ContainsItem _targetsinrange (Variables|Default|GetTargetEnemyDetected))
          (Utilities|Array|RemoveItem _targetsinrange (Variables|Default|GetTargetEnemyDetected))
          (Variables|Default|SetTargetEnemyDetected 0)
          (CallFunction|SelectTarget))))
    (:Is%20Not%20Valid
      (goto _label))))

(event Custom|CancelAim
  ;[1 1 1] Vise
  (Utilities|FlowControl|Gate true) ; enters at Close
)

(event EventTick
  (params (DeltaSeconds :type Float%20%28single-precision%29))
  (bind _returnvalue (Game|GetPlayerController 0))
  (bind (_worldlocation _worlddirection) (Game|Player|ConvertMouseLocationToWorldSpace _returnvalue))
  (bind _z (Math|Vector|BreakVector _worldlocation))
  (bind _z_2 (Math|Vector|BreakVector _worlddirection))
  (bind _returnvalue_2 (/ _z _z_2))
  (bind _returnvalue_3 (* _worlddirection _returnvalue_2))
  (bind _returnvalue_4 (* _returnvalue_3 -1.0))
  (bind _returnvalue_5 (+ _worldlocation _returnvalue_4))
  ;[1 1 1] Click and Drop
  (if (not (Variables|Default|GetPlaced))
    (Transformation|SetActorLocation (Math|Vector|MakeVector (.x _returnvalue_5) (.y _returnvalue_5) 1.5e+02) false false)))

(fn ConstructionScript)

(fn Shot
  (params (ProjectyleType :type BP%20Projectiles%20Parent%20Class%20Reference))
  (bind _returnvalue (Game|SpawnActorfromClass ProjectyleType (Transformation|GetWorldTransform (Variables|Default|GetCannon)) "Undefined" 0 0))
  (Variables|Default|SetProjectyle _returnvalue))

(fn Shot3
  (params (ProjectyleType :type BP%20Projectiles%20Parent%20Class%20Reference))
  (bind _cannon2 (Variables|Default|GetCannon2))
  (bind _cannon3 (Variables|Default|GetCannon3))
  (bind _returnvalue (Transformation|GetWorldTransform _cannon2))
  (bind _returnvalue_2 (Transformation|GetWorldTransform _cannon3))
  (Utilities|FlowControl|Sequence
    (:then_0
      (Game|SpawnActorfromClass ProjectyleType (Transformation|GetWorldTransform (Variables|Default|GetCannon)) "Undefined" 0 0))
    (:then_1
      (Game|SpawnActorfromClass ProjectyleType (Math|Transform|MakeTransform (.location _returnvalue) (Math|Rotator|MakeRotator (.roll (.rotation _returnvalue)) (.pitch (.rotation _returnvalue)) (+ (.yaw (.rotation _returnvalue)) 45.0)) (.scale _returnvalue)) "Undefined" 0 0))
    (:then_2
      (Game|SpawnActorfromClass ProjectyleType (Math|Transform|MakeTransform (.location _returnvalue_2) (Math|Rotator|MakeRotator (.roll (.rotation _returnvalue_2)) (.pitch (.rotation _returnvalue_2)) (+ (.yaw (.rotation _returnvalue_2)) -45.0)) (.scale _returnvalue_2)) "Undefined" 0 0))))

(fn DamageAura)